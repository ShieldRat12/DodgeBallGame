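; AI catch partner that destroys any actor overlapping its capsule, then after a delay throws a new BP_CatchBall.
; BeginPlay attaches it to BP_Platform2 and caches the first-person player, whose location is sampled per throw while a catch count increments.
; The ball spawns at ThrowingSpot and receives a ThrowingSuff_3 impulse, with projectile movement toggled briefly.
; ThrowingSuff_3 holds only unconnected ballistic-arc and straight-line calculations.
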(event OnComponentBeginOverlap(CapsuleComponent)
  (params (OverlappedComponent :type Primitive%20Component%20Object%20Reference) (OtherActor :type Actor%20Object%20Reference) (OtherComp :type Primitive%20Component%20Object%20Reference) (OtherBodyIndex :type Integer) (bFromSweep :type Boolean) (SweepResult :type Hit%20Result%20Structure%20%28by%20ref%29))
  (Actor|DestroyActor OtherActor)
  (Utilities|FlowControl|Delay 2.0)
  (CallFunction|GetTargetLocation)
  (bind _returnvalue (Game|SpawnActorfromClass "/Game/DodgeBalls/BP_CatchBall.BP_CatchBall_C" (Transformation|GetWorldTransform (Variables|Default|GetThrowingSpot)) "AlwaysSpawn" "MultiplyWithRoot" 0 0))
  (Components|Activation|Activate (Variables|/Game/DodgeBalls/BP_CatchBall.BP_CatchBall_C|GetProjectileMovement _returnvalue) false)
  (Physics|AddImpulse (Variables|/Game/DodgeBalls/BP_CatchBall.BP_CatchBall_C|GetStaticMesh _returnvalue) (|Throwingsuff_3) "None" false)
  (Utilities|FlowControl|Delay 0.0001)
  (Components|Activation|Deactivate (Variables|/Game/DodgeBalls/BP_CatchBall.BP_CatchBall_C|GetProjectileMovement _returnvalue)))

(event Custom|GetTargetLocation
  (bind _fpc (Variables|Default|GetFPC)
    (:then
      (Variables|Default|SetFPCLocation (Transformation|GetActorLocation _fpc))
      (bind _result (Math|Integer|IncrementInt (Variables|Default|GetCatchCount))
        (:%20%20
          (bind _output_get (Variables|Default|SetCatchCount _result))
          (Development|PrintString (Utilities|String|ToString(Integer) _output_get)))))
    (:else)))

(event EventBeginPlay
  (bind _returnvalue (Actor|GetActorOfClass "/Game/CatchStuff/BP_Platform2.BP_Platform2_C"))
  (Transformation|AttachComponentToComponent (Variables|/Game/CatchStuff/BP_Platform2.BP_Platform2_C|GetDefaultSceneRoot _returnvalue) "None" "KeepWorld" "KeepRelative" "KeepRelative" true)
  (bind _returnvalue_2 (Actor|GetActorOfClass "/Game/People_Players/FirstPerson/Blueprints/BP_FirstPersonCharacter_Catch.BP_FirstPersonCharacter_Catch_C"))
  (Variables|Default|SetFPC _returnvalue_2)
  (Variables|Default|GetFPC
    (:then)
    (:else)))

(fn ConstructionScript)