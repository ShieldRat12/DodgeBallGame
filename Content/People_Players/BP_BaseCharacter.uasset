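; BP_BaseCharacter is a base character Blueprint that provides health, damage and death handling.
; TakeDamage subtracts damage from Health, clamps it between zero and MaxHealth, and triggers Dead once at zero, guarded by the IsDead flag.
; Dead ragdolls the mesh with physics and blocking collision, stops movement, then destroys the actor after a short delay.
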(event Custom|TakeDamage
  (params (Damage :type Float%20%28double-precision%29))
  (if (not (Variables|Default|GetIsDead))
    (bind _output_get (Variables|Default|SetHealth (Math|Float|Clamp(Float) (- (Variables|Default|GetHealth) Damage) 0.0 (Variables|Default|GetMaxHealth))))
    (if (<= _output_get 0.0)
      (Variables|Default|SetIsDead true)
      (CallFunction|Dead))))

(event Custom|Dead
  (bind _mesh (Variables|Character|GetMesh))
  (Physics|SetSimulatePhysics _mesh true)
  (Components|Movement|StopMovementImmediately (Variables|Character|GetCharacterMovement))
  (Collision|SetCollisionProfileName _mesh "BlockAllDynamic" true :!class /Script/Engine.PrimitiveComponent)
  (Utilities|FlowControl|Delay 3.0)
  (Actor|DestroyActor))

(event EventBeginPlay)

(event Collision|EventActorBeginOverlap
  (params (OtherActor :type Actor%20Object%20Reference)))

(event EventTick
  (params (DeltaSeconds :type Float%20%28single-precision%29)))

(fn ConstructionScript)