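; Parent dodgeball Blueprint that damages characters on hit and supports being caught.
; On sphere overlap it records ball speed, waits briefly, then, unless caught, deals speed-tiered damage to the overlapped BP_BaseCharacter.
; CatchLogic uses that stored speed to set a Multiplier and the IsCaught flag that cancels damage.
; The middle catch tier is unreachable because its condition repeats the top tier's threshold.
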(event OnComponentBeginOverlap(SphereCollision)
  (params (OverlappedComponent :type Primitive%20Component%20Object%20Reference) (OtherActor :type Actor%20Object%20Reference) (OtherComp :type Primitive%20Component%20Object%20Reference) (OtherBodyIndex :type Integer) (bFromSweep :type Boolean) (SweepResult :type Hit%20Result%20Structure%20%28by%20ref%29))
  (Variables|Default|SetHitTarget OtherActor)
  (bind _output_get (Variables|Default|SetBallSpeed (Math|Vector|VectorLength (Transformation|GetComponentVelocity (Variables|Default|GetStaticMesh)))))
  (Utilities|FlowControl|Delay 0.05)
  (if (not (Variables|Default|GetIsCaught))
    (if (>= _output_get 6e+03)
      (bind _asbp_base_character (Utilities|Casting|CastToBP_BaseCharacter (Variables|Default|GetHitTarget)))
      (Default|TakeDamage _asbp_base_character 8e+01)
      (Development|PrintString "80")
      (elif (>= _output_get 5e+03)
        (bind _asbp_base_character_2 (Utilities|Casting|CastToBP_BaseCharacter (Variables|Default|GetHitTarget)))
        (Default|TakeDamage _asbp_base_character_2 6e+01)
        (Development|PrintString "60")
        (elif (>= _output_get 4.5e+03)
          (bind _asbp_base_character_3 (Utilities|Casting|CastToBP_BaseCharacter (Variables|Default|GetHitTarget)))
          (Default|TakeDamage _asbp_base_character_3 4e+01)
          (Development|PrintString "40")
          (elif (>= _output_get 1.2e+03)
            (bind _asbp_base_character_4 (Utilities|Casting|CastToBP_BaseCharacter (Variables|Default|GetHitTarget)))
            (Default|TakeDamage _asbp_base_character_4 2e+01)
            (Development|PrintString "20")))))
    (else
      (Development|PrintString "No damage"))))

(fn ConstructionScript)

(fn CatchLogic
  (bind _ballspeed (Variables|Default|GetBallSpeed))
  (if (> (Variables|Default|GetBallSpeed) 1.5e+03)
    (Development|PrintString "Catchable 3")
    (Variables|Default|SetMultiplier 4.0)
    (Variables|Default|SetIsCaught true :!label _label)
    (elif (and (< 1.5e+03 _ballspeed) (> _ballspeed 6e+02))
      (Development|PrintString "Catchable 2")
      (Variables|Default|SetMultiplier 2.5)
      (goto _label)
      (elif (< 2e+02 (Variables|Default|GetBallSpeed))
        (Development|PrintString "Catchable 1")
        (Variables|Default|SetMultiplier 1.5)
        (goto _label)))))